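; BP_Terminal is a terminal actor that displays its widget only while the first-person player character is nearby.
; The TerminalWidget component's user widget starts hidden on BeginPlay.
; A Sphere component's begin and end overlap events, filtered by a cast to BP_FirstPersonCharacter, toggle that widget between visible and hidden.
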(event OnComponentBeginOverlap(Sphere)
  (params (OverlappedComponent :type Primitive%20Component%20Object%20Reference) (OtherActor :type Actor%20Object%20Reference) (OtherComp :type Primitive%20Component%20Object%20Reference) (OtherBodyIndex :type Integer) (bFromSweep :type Boolean) (SweepResult :type Hit%20Result%20Structure%20%28by%20ref%29))
  (Utilities|Casting|CastToBP_FirstPersonCharacter OtherActor)
  (Widget|SetVisibility (UserInterface|GetWidget (Variables|Default|GetTerminalWidget)) "Visible"))

(event OnComponentEndOverlap(Sphere)
  (params (OverlappedComponent :type Primitive%20Component%20Object%20Reference) (OtherActor :type Actor%20Object%20Reference) (OtherComp :type Primitive%20Component%20Object%20Reference) (OtherBodyIndex :type Integer))
  (Utilities|Casting|CastToBP_FirstPersonCharacter OtherActor)
  (Widget|SetVisibility (UserInterface|GetWidget (Variables|Default|GetTerminalWidget)) "Hidden"))

(event EventBeginPlay
  (Widget|SetVisibility (UserInterface|GetWidget (Variables|Default|GetTerminalWidget)) "Hidden"))

(fn ConstructionScript)
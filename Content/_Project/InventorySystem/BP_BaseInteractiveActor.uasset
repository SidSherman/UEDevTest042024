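; Base actor Blueprint for interactive objects in the inventory system.
; Handles Interact, StopInteract and Lookat events with placeholder debug prints naming the actor, plus the interactor on Interact.
; The look-at print uses a fixed key, so repeated calls replace one on-screen message instead of stacking.
; BeginPlay, overlap, Tick and the construction script are empty.
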(event EventBeginPlay)

(event Collision|EventActorBeginOverlap
  (params (OtherActor :type Actor%20Object%20Reference)))

(event EventTick
  (params (DeltaSeconds :type Float%20%28single-precision%29)))

(event EventInteract
  (params (Interactor :type Actor%20Object%20Reference))
  (Development|PrintText (Utilities|Text|FormatText "Start Interact 
Interactor: {0} 
Actor: {1}" (Utilities|GetDisplayName Interactor) (Utilities|GetDisplayName self))))

(event EventStopInteract
  (Development|PrintText (Utilities|Text|FormatText "Stop Interact 
Actor: {1}" (Utilities|GetDisplayName self))))

(event EventLookat
  (params (Interactor :type Actor%20Object%20Reference))
  (Development|PrintText (Utilities|Text|FormatText "LookAt 
Actor: {1}" (Utilities|GetDisplayName self)) true true "(R=0.000000,G=0.660000,B=1.000000,A=1.000000)" 2.0 "LookAtDebug"))

(fn ConstructionScript)
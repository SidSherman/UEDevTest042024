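; Inventory component for the first-person character that stores items in fixed-size slots and lets the player hold or drop them.
; Adding looks for a non-full matching slot using DT_ItemData stack sizes, else an empty one, though AddToStack overwrites quantity instead of incrementing.
; Selecting a slot shows its stored actor, or spawns one from the data table, for grabbing; deselecting hides or destroys it.
; Changes refresh BP_BaseHUD.
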(event EventBeginPlay
  ;[1 1 1] InitArray
  (Utilities|Array|Resize (Variables|Default|GetContent) (Variables|Default|GetInventorySize))
  (CallFunction|UpdateUI))

(event Input|KeyboardEvents|I
  (params (Key :type Key%20Structure))
  ;[1 1 1] Debug
  (:Pressed
    (for (_array_element _array_index) (Variables|Default|GetContent)
      (Development|PrintText (Utilities|Text|FormatText "Item ID {0} | Item Quantity {1} | Slot {2}" (.itemid _array_element) (.quantity _array_element) _array_index)))))

(fn AddtoInventory
  (params (ItemID :type Name) (Quantity :type Integer) (Actors :type Array%20of%20BP%20Interactive%20Inventory%20Item%20Object%20Object%20References))
  (LocalVariables|SetLocalQuanityRemaining Quantity)
  (while (and (> (LocalVariables|GetLocalQuanityRemaining) 0) (not (LocalVariables|GetbHasLocalFailed)))
    (bind (_array_index _bisfoundslot) (CallFunction|FindSlot ItemID))
    (if _bisfoundslot
      (CallFunction|AddtoStack _array_index 1 Actors)
      (Math|Integer|DecrementInt (LocalVariables|GetLocalQuanityRemaining))
      (elif (.bHasEmptySlot (CallFunction|FindAnyEmptySlotsAvaliable))
        (bind _bissuccessed (CallFunction|CreateStack ItemID 1 Actors))
        (if _bissuccessed
          (Math|Integer|DecrementInt (LocalVariables|GetLocalQuanityRemaining))
          (else
            (LocalVariables|SetbHasLocalFailed true)))
        (else
          (LocalVariables|SetbHasLocalFailed true)))))
  (CallFunction|UpdateUI)
  (return (not (LocalVariables|GetbHasLocalFailed)) (LocalVariables|GetLocalQuanityRemaining)))

(fn RemovefromInventory
  (params (SlotId :type Integer) (RemoveWholeStack :type Boolean))
  (bind _content (Variables|Default|GetContent))
  (bind _output (Utilities|Array|Get(acopy) _content SlotId))
  (bind _returnvalue (Utilities|Array|Length (.actor _output)))
  (bind _returnvalue_2 (- _returnvalue 1))
  (if (Utilities|Array|IsValidIndex (Variables|Default|GetContent) SlotId)
    (if RemoveWholeStack
      (Utilities|Array|SetArrayElem (Variables|Default|GetContent) SlotId (Utilities|Struct|MakeFSlotStruct "None" 0 0))
      (else
        (bind _result (Math|Integer|DecrementInt (.quantity _output))
          (:%20%20
            (bind _asbp_first_person_character (Utilities|Casting|CastToBP_FirstPersonCharacter (Components|GetOwner))
              (:then
                (Default|ShowItem (Utilities|Array|Get(acopy) (.actor _output) _returnvalue_2) (Default|GetPointinFrontOf _asbp_first_person_character 1e+02) "0, 0, 0"))
              (:CastFailed
                _))
            (Utilities|Array|RemoveIndex (.actor _output) _returnvalue_2)
            (Utilities|Array|SetArrayElem (Variables|Default|GetContent) SlotId (Utilities|Struct|MakeFSlotStruct (.itemid _output) (Math|Integer|Clamp(Integer) _result 0 (.quantity _output)) (.actor _output)))))))
    (CallFunction|UpdateUI)))

(fn FindSlot
  (params (ItemID :type Name))
  (for (_array_element _array_index) (Variables|Default|GetContent)
    (if (== (.itemid _array_element) ItemID)
      (if (< (.quantity _array_element) (CallFunction|GetMaxStackSize ItemID))
        (return _array_index true))))
  (return -1 false))

(fn GetMaxStackSize
  (params (ItemId :type Name))
  (bind _returnvalue (Utilities|GetDataTableRow "/Game/_Project/Data/DT_ItemData.DT_ItemData" ItemId)
    (:then
      (return (.stacksize _returnvalue)))
    (:RowNotFound
      (return -1))))

(fn AddtoStack
  (params (Index :type Integer) (Quantity :type Integer) (Actors :type Array%20of%20BP%20Interactive%20Inventory%20Item%20Object%20Object%20References))
  (Utilities|Array|SetArrayElem (Variables|Default|GetContent) Index (Utilities|Struct|MakeFSlotStruct (.itemid (Utilities|Array|Get(acopy) (Variables|Default|GetContent) Index)) Quantity Actors)))

(fn FindAnyEmptySlotsAvaliable
  (for (_array_element _array_index) (Variables|Default|GetContent)
    (if (== (.quantity _array_element) 0)
      (return true _array_index)))
  (return false -1))

(fn CreateStack
  (params (ItemId :type Name) (Quanitity :type Integer) (Actors :type Array%20of%20BP%20Interactive%20Inventory%20Item%20Object%20Object%20References))
  (bind (_bhasemptyslot _array_index) (CallFunction|FindAnyEmptySlotsAvaliable))
  (if _bhasemptyslot
    (Utilities|Array|SetArrayElem (Variables|Default|GetContent) _array_index (Utilities|Struct|MakeFSlotStruct ItemId Quanitity Actors))
    (return true)
    (else
      (return false))))

(fn SelectItem
  (params (SlotId :type Integer))
  (Utilities|FlowControl|Sequence
    (:then_0
      (LocalVariables|SetPrevSelectedItemId (Variables|Default|GetSelectedItem))
      (if (== SlotId (Variables|Default|GetSelectedItem))
        (CallFunction|RemoveActor)
        (Variables|Default|SetSelectedItem -1)
        (else
          (CallFunction|RemoveActor)
          (bind _output_get (Variables|Default|SetSelectedItem SlotId))
          (CallFunction|CreateActor _output_get))))
    (:then_1
      (bind _asbp_base_hud (Utilities|Casting|CastToBP_BaseHUD (HUD|GetHUD (Game|GetPlayerController 0))))
      (Default|UpdateHUD _asbp_base_hud))))

(fn CreateActor
  (params (SlotId :type Integer))
  (bind _returnvalue (Components|GetOwner))
  (bind _content (Variables|Default|GetContent))
  (bind _content_2 (Variables|Default|GetContent))
  (bind _selecteditem (Variables|Default|GetSelectedItem))
  (bind _output (Utilities|Array|Get(acopy) _content_2 _selecteditem))
  (bind _output_2 (Utilities|Array|Get(acopy) (.actor _output)))
  (Utilities|FlowControl|Sequence
    (:then_0
      (bind _asbp_first_person_character (Utilities|Casting|CastToBP_FirstPersonCharacter (Components|GetOwner)))
      (LocalVariables|SetFirstPersonChar _asbp_first_person_character))
    (:then_1
      (if (Utilities|Array|IsValidIndex _content_2 _selecteditem)
        (if (Utilities|Array|IsValidIndex (.actor _output))
          (bind _firstpersonchar (LocalVariables|GetFirstPersonChar)
            (:then
              (Utilities|IsValid _output_2
                (:Is%20Valid
                  (Actor|SetOwner _output_2 _firstpersonchar)
                  (Default|ShowItem _output_2 (Default|GetPointinFrontOf _firstpersonchar 5e+01) "0, 0, 0")
                  (bind _output_get (Variables|Default|SetGrabbedActor _output_2))
                  (bind _firstpersonchar_2 (LocalVariables|GetFirstPersonChar)
                    (:then
                      (Default|GrabActor _firstpersonchar_2 (Variables|Default|GetGrabbedActor) (Variables|/Game/_Project/InventorySystem/BP_BaseInteractiveActor.BP_BaseInteractiveActor_C|GetStaticMesh _output_get)))
                    (:else)))
                (:Is%20Not%20Valid
                  (bind _firstpersonchar_3 (LocalVariables|GetFirstPersonChar)
                    (:then
                      (Variables|/Game/FirstPerson/Blueprints/BP_FirstPersonCharacter.BP_FirstPersonCharacter_C|SetInteractive%20Hit%20Actor _firstpersonchar_3 0))
                    (:else)))))
            (:else))
          (else
            (if (Utilities|Array|IsValidIndex _content SlotId) :!label _label
              (bind _returnvalue_2 (Utilities|GetDataTableRow "/Game/_Project/Data/DT_ItemData.DT_ItemData" (.itemid (Utilities|Array|Get(acopy) _content SlotId)))
                (:then
                  (bind _returnvalue_3 (Game|SpawnActorfromClass (.ItemClass (Utilities|Struct|BreakFItemStruct _returnvalue_2)) (Math|Transform|MakeTransform (select (Utilities|IsValid (LocalVariables|GetFirstPersonChar)) (Default|GetPointinFrontOf (LocalVariables|GetFirstPersonChar) 5e+01) (+ (Transformation|GetActorLocation _returnvalue) (* (Math|Vector|GetForwardVector (Transformation|GetWorldRotation (Variables|/Script/Engine.Actor|GetRootComponent _returnvalue))) 5e+01))) "0, 0, 0" "1.000000,1.000000,1.000000") "AdjustIfPossibleButAlwaysSpawn" "MultiplyWithRoot" (Components|GetOwner) 0))
                  (bind _asbp_interactive_inventory_item_object (Utilities|Casting|CastToBP_InteractiveInventoryItemObject _returnvalue_3))
                  (bind _output_get_2 (Variables|Default|SetGrabbedActor _asbp_interactive_inventory_item_object))
                  (bind _firstpersonchar_4 (LocalVariables|GetFirstPersonChar)
                    (:then
                      (Actor|SetOwner _output_get_2 _firstpersonchar_4)
                      (Default|GrabActor _firstpersonchar_4 (Variables|Default|GetGrabbedActor) (Variables|/Game/_Project/InventorySystem/BP_BaseInteractiveActor.BP_BaseInteractiveActor_C|GetStaticMesh _output_get_2)))
                    (:else)))
                (:RowNotFound
                  (bind _firstpersonchar_5 (LocalVariables|GetFirstPersonChar)
                    (:then
                      (Variables|/Game/FirstPerson/Blueprints/BP_FirstPersonCharacter.BP_FirstPersonCharacter_C|SetInteractive%20Hit%20Actor _firstpersonchar_5 0))
                    (:else)))))))
        (else
          (goto _label))))))

(fn RemoveActor
  (bind _content (Variables|Default|GetContent))
  (bind _selecteditem (Variables|Default|GetSelectedItem))
  (bind _output (Utilities|Array|Get(acopy) _content _selecteditem))
  (bind _output_2 (Utilities|Array|Get(acopy) (.actor _output)))
  (if (Utilities|Array|IsValidIndex _content _selecteditem)
    (if (Utilities|Array|IsValidIndex (.actor _output))
      (Utilities|IsValid _output_2
        (:Is%20Valid
          (Default|HideItem _output_2)
          (Utilities|FlowControl|Sequence
            (:then_0
              (bind _grabbedactor (Variables|Default|GetGrabbedActor)
                (:then
                  (Actor|SetOwner _grabbedactor 0)
                  (Variables|Default|SetGrabbedActor 0))
                (:else)))
            (:then_1
              (bind _asbp_first_person_character (Utilities|Casting|CastToBP_FirstPersonCharacter (Components|GetOwner)))
              (Default|UnGrab _asbp_first_person_character)))))
      (else
        (bind _grabbedactor_2 (Variables|Default|GetGrabbedActor :!label _label)
          (:then
            (Actor|DestroyActor _grabbedactor_2))
          (:else))))
    (else
      (goto _label))))

(fn DropSelectedItem
  (if (Utilities|Array|IsValidIndex (Variables|Default|GetContent) (Variables|Default|GetSelectedItem))
    (Utilities|FlowControl|Sequence
      (:then_0
        (CallFunction|RemovefromInventory (Variables|Default|GetSelectedItem) true)
        (Variables|Default|SetSelectedItem -1)
        (CallFunction|UpdateUI))
      (:then_1
        (bind _asbp_first_person_character (Utilities|Casting|CastToBP_FirstPersonCharacter (Components|GetOwner)))
        (bind _output_get (LocalVariables|SetFirstPersonChar _asbp_first_person_character))
        (Default|UnGrab _output_get)
        (Variables|Default|SetGrabbedActor 0)))))

(fn UpdateUI
  (bind _asbp_base_hud (Utilities|Casting|CastToBP_BaseHUD (HUD|GetHUD (Game|GetPlayerController 0))))
  (Default|UpdateHUD _asbp_base_hud))

(fn CanGrabSomeItem
  (return (not (Utilities|IsValid (Variables|Default|GetGrabbedActor)))))
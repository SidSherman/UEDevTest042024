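; Interactive world item that an interactor with an inventory component can pick up into its inventory.
; On interact, it passes its item data component's ID and quantity plus itself to the inventory, then hides instead of being destroyed.
; ShowItem and HideItem toggle physics, collision and visibility, with ShowItem also repositioning the actor.
; Look-at prints data table name and description as debug text; grabbing ignores Pawn and a custom collision channel.
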(event EventBeginPlay
  (|CallParentFunction) ; This node is disabled and will not be called.\nDrag off pins to build functionality.
)

(event Collision|EventActorBeginOverlap
  (params (OtherActor :type Actor%20Object%20Reference))
  (|CallParentFunction OtherActor) ; This node is disabled and will not be called.\nDrag off pins to build functionality.
)

(event EventTick
  (params (DeltaSeconds :type Float%20%28single-precision%29))
  (|CallParentFunction DeltaSeconds) ; This node is disabled and will not be called.\nDrag off pins to build functionality.
)

(event EventInteract
  (params (Interactor :type Actor%20Object%20Reference))
  (bind _returnvalue (Actor|GetComponentbyClass Interactor "/Game/_Project/InventorySystem/BPC_InventoryComponent.BPC_InventoryComponent_C"))
  (bind _bpc_itemdatacomponent (Variables|Default|GetBPC_ItemDataComponent))
  (|CallParentFunction Interactor)
  (Utilities|IsValid _returnvalue
    (:Is%20Valid
      (if (Default|CanGrabSomeItem _returnvalue)
        (bind _bhassuccessed (Default|AddtoInventory _returnvalue (.rowname (Variables|/Game/_Project/InventorySystem/BPC_ItemDataComponent.BPC_ItemDataComponent_C|GetItemID _bpc_itemdatacomponent)) (Variables|/Game/_Project/InventorySystem/BPC_ItemDataComponent.BPC_ItemDataComponent_C|GetQuantity _bpc_itemdatacomponent) (Utilities|Array|MakeArray self)))
        (if _bhassuccessed
          (CallFunction|HideItem)
          (bind _asbp_first_person_character (Utilities|Casting|CastToBP_FirstPersonCharacter Interactor))
          (Variables|/Game/FirstPerson/Blueprints/BP_FirstPersonCharacter.BP_FirstPersonCharacter_C|SetInteractive%20Hit%20Actor _asbp_first_person_character 0))))))

(event EventStopInteract
  (|CallParentFunction))

(event EventLookat
  (params (Interactor :type Actor%20Object%20Reference))
  (bind _bpc_itemdatacomponent (Variables|Default|GetBPC_ItemDataComponent))
  (bind _itemid (Variables|/Game/_Project/InventorySystem/BPC_ItemDataComponent.BPC_ItemDataComponent_C|GetItemID _bpc_itemdatacomponent))
  (|CallParentFunction Interactor)
  (bind _returnvalue (Utilities|GetDataTableRow (.datatable _itemid) (.rowname _itemid))
    (:then
      (Development|PrintText (Utilities|Text|FormatText "Inventory Item Nane: {0} 
Description: {1}" (.Name (Utilities|Struct|BreakFItemStruct _returnvalue)) (.Description (Utilities|Struct|BreakFItemStruct _returnvalue))) true true "(R=0.000000,G=0.660000,B=1.000000,A=1.000000)" 2.0 "IvenetoryItemLookAtDebug"))))

(event EventGrab
  (params (bIsGrab :type Boolean))
  (bind _returnvalue (select bIsGrab "ECR_Ignore" "ECR_Block"))
  (bind _staticmesh (Variables|Default|GetStaticMesh))
  (|CallParentFunction bIsGrab)
  (Utilities|FlowControl|Sequence
    (:then_0
      (Collision|SetCollisionResponsetoChannel _staticmesh "ECC_GameTraceChannel3" _returnvalue)
      (Collision|SetCollisionResponsetoChannel _staticmesh "ECC_Pawn" _returnvalue))))

(fn ConstructionScript
  (|CallParentFunction))

(fn ShowItem
  (params (Dest :type Vector) (Rotarion :type Rotator))
  (bind _staticmesh (Variables|Default|GetStaticMesh))
  (Transformation|SetActorLocationAndRotation Dest (Math|Rotator|SelectRotator (Transformation|GetActorRotation) Rotarion (Utilities|Operators|EqualEqual :A Rotarion :ErrorTolerance 0.1)))
  (Physics|SetSimulatePhysics _staticmesh true)
  (Collision|SetCollisionEnabled _staticmesh "QueryAndPhysics")
  (Rendering|SetVisibility (Variables|Default|GetStaticMesh) true true))

(fn HideItem
  (bind _staticmesh (Variables|Default|GetStaticMesh))
  (Physics|SetSimulatePhysics _staticmesh false)
  (Collision|SetCollisionEnabled _staticmesh "NoCollision")
  (Rendering|SetVisibility (Variables|Default|GetStaticMesh) false true))